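; Player controller that runs the NPC dialogue UI and adds the default Enhanced Input mapping context on BeginPlay.
; DialogueTrigger disables player input, creates the dialogue widget if needed, switches to UI-only input and fills in name, text and options.
; When options exist, it rebinds a dispatcher to the caller's event, which ClickButton fires after storing the chosen option.
; CloseDialogue removes the widget and restores game input.
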(event EventBeginPlay
  (bind _returnvalue (PlayerController|LocalPlayerSubsystems|GetEnhancedInputLocalPlayerSubsystem))
  (Utilities|IsValid _returnvalue
    (:Is%20Valid
      (Input|AddMappingContext _returnvalue "/Game/FirstPerson/Input/IMC_Default.IMC_Default" 0 "(bIgnoreAllPressedKeysUntilRelease=True,bForceImmediately=False,bNotifyUserSettings=False)"))))

(fn ConstructionScript)

(fn ClickButton
  (params (CurrentOption :type Integer))
  (Variables|Default|SetCurrent%20Option CurrentOption)
  (Default|CallDialogueTrigger))

(fn DialogueTrigger
  (params (Event :type Delegate%20%28by%20ref%29) (NewParam :type Every%20Talk%20Structure))
  (bind (_npc_name _dialogue_text _options) (Utilities|Struct|BreakEveryTalk NewParam))
  (Input|DisableInput self 0)
  (Variables|Default|GetDialogue_Interface
    (:then
      _)
    (:else
      (bind _returnvalue (UserInterface|CreateWidget "/Game/Level1/NPC/WB_Dialogue_Interface.WB_Dialogue_Interface_C"))
      (bind _output_get (Variables|Default|SetDialogue_Interface _returnvalue))
      (UserInterface|Viewport|AddtoViewport _output_get 0)
      (Input|SetInputModeUIOnly self _output_get "DoNotLock" false)
      (Variables|Default|SetbShowMouseCursor true)))
  (Utilities|FlowControl|Sequence
    (:then_0
      (Variables|/Script/UMG.TextBlock|SetText (Variables|/Game/Level1/NPC/WB_Dialogue_Interface.WB_Dialogue_Interface_C|GetNPC_Name (Variables|Default|GetDialogue_Interface)) _npc_name)
      (Variables|/Script/UMG.TextBlock|SetText (Variables|/Game/Level1/NPC/WB_Dialogue_Interface.WB_Dialogue_Interface_C|GetDialogue_Text (Variables|Default|GetDialogue_Interface)) (Utilities|Text|ToText(String) _dialogue_text)))
    (:then_1
      (if (Utilities|Array|IsNotEmpty _options)
        (EventDispatchers|UnbindallEventsfromDialogueTrigger)
        (EventDispatchers|BindEventtoDialogueTrigger Event)
        (Default|AddOptions (Variables|Default|GetDialogue_Interface) _options)))))

(fn CloseDialogue
  (Input|EnableInput self 0)
  (Widget|RemovefromParent (Variables|Default|GetDialogue_Interface))
  (Variables|Default|SetDialogue_Interface 0)
  (Variables|Default|SetbShowMouseCursor false)
  (Input|SetInputModeGameOnly self false))