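; BP_NPC_Test is the M&M NPC for Level 1 that opens a branching escape-room dialogue when the player overlaps its sphere.
; Chained events pass each next step to BP_Dialogue_Sys; the final branches start the HUD and world countdown clocks and set the player's HasStarted.
; The polite branch grants a longer timer than the rude one, but event 2 switches on a constant 0, leaving the rude branch unreachable.
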(event OnComponentBeginOverlap(Sphere)
  (params (OverlappedComponent :type Primitive%20Component%20Object%20Reference) (OtherActor :type Actor%20Object%20Reference) (OtherComp :type Primitive%20Component%20Object%20Reference) (OtherBodyIndex :type Integer) (bFromSweep :type Boolean) (SweepResult :type Hit%20Result%20Structure%20%28by%20ref%29))
  (if (== OtherActor (Variables|Default|GetAs%20BP%20First%20Person%20Character))
    (Default|DialogueTrigger (Variables|Default|GetAs%20BP%20Dialogue%20Sys) (delegate Custom|1) (Utilities|Struct|MakeEveryTalk "M&M" "Do u feel good? This is the place you've been living for years... 
But this is only your dream..and it is collapsing... 
Get out! ...before you can..." (Utilities|Array|MakeArray "But how can I get out" "Yeah yeah yeah I know it")))))

(event Custom|1
  (switch int (Variables|/Game/Level1/NPC/BP_Dialogue_Sys.BP_Dialogue_Sys_C|GetCurrent%20Option (Variables|Default|GetAs%20BP%20Dialogue%20Sys))
    (:0
      (Default|DialogueTrigger (Variables|Default|GetAs%20BP%20Dialogue%20Sys) (delegate Custom|2) (Utilities|Struct|MakeEveryTalk "M&M" "You will find some clues in this room...but not everything is clue! 
They might be fake...hahaha 
I can give u one: You need to find a key！~" (Utilities|Array|MakeArray "Thank you so much!" "You ugly face! I'm not stupid!"))))
    (:1
      (Default|CloseDialogue (Variables|Default|GetAs%20BP%20Dialogue%20Sys)))))

(event Custom|2
  (switch int 0
    (:0
      (Default|DialogueTrigger (Variables|Default|GetAs%20BP%20Dialogue%20Sys) (delegate Custom|3_1) (Utilities|Struct|MakeEveryTalk "M&M" "You are nice too... Good luck!" (Utilities|Array|MakeArray "I will try my best!"))))
    (:1
      (Default|DialogueTrigger (Variables|Default|GetAs%20BP%20Dialogue%20Sys) (delegate Custom|3_2) (Utilities|Struct|MakeEveryTalk "M&M" "You are so rude.......you deserve it...Heh heh" (Utilities|Array|MakeArray "Such a weirdo!"))))))

(event Custom|3_1
  (bind _countdownwidgetref (Variables|Default|GetCountdownWidgetRef))
  (bind _countdown_clock (Variables|Default|GetCountdown%20Clock))
  (switch int (Variables|/Game/Level1/NPC/BP_Dialogue_Sys.BP_Dialogue_Sys_C|GetCurrent%20Option (Variables|Default|GetAs%20BP%20Dialogue%20Sys))
    (:0
      (Default|CloseDialogue (Variables|Default|GetAs%20BP%20Dialogue%20Sys))
      (if (not (Variables|/Game/Level1/Countdown/BP_CountdownTimer.BP_CountdownTimer_C|GetIsCountingDown _countdownwidgetref))
        (Variables|/Game/Level1/Countdown/BP_CountdownTimer.BP_CountdownTimer_C|SetIsCountingDown _countdownwidgetref true)
        (Default|SetDuration _countdownwidgetref 3e+02)
        (UserInterface|Viewport|AddtoViewport _countdownwidgetref 0)
        (if (not (Variables|/Game/Level1/Inventory/Items/BP_Countdown_Clock.BP_Countdown_Clock_C|GetIsCountingDown _countdown_clock))
          (Default|SetDuration _countdown_clock 3e+02)
          (Variables|/Game/Level1/Inventory/Items/BP_Countdown_Clock.BP_Countdown_Clock_C|SetIsCountingDown _countdown_clock true)
          (Variables|/Game/FirstPerson/Blueprints/BP_FirstPersonCharacter.BP_FirstPersonCharacter_C|SetHasStarted (Variables|Default|GetAs%20BP%20First%20Person%20Character) true))))))

(event Custom|3_2
  (bind _countdown_clock (Variables|Default|GetCountdown%20Clock))
  (bind _countdownwidgetref (Variables|Default|GetCountdownWidgetRef))
  (switch int (Variables|/Game/Level1/NPC/BP_Dialogue_Sys.BP_Dialogue_Sys_C|GetCurrent%20Option (Variables|Default|GetAs%20BP%20Dialogue%20Sys))
    (:0
      (Default|CloseDialogue (Variables|Default|GetAs%20BP%20Dialogue%20Sys))
      (if (not (Variables|/Game/Level1/Countdown/BP_CountdownTimer.BP_CountdownTimer_C|GetIsCountingDown _countdownwidgetref))
        (Variables|/Game/Level1/Countdown/BP_CountdownTimer.BP_CountdownTimer_C|SetIsCountingDown _countdownwidgetref true)
        (Default|SetDuration _countdownwidgetref 1.2e+02)
        (UserInterface|Viewport|AddtoViewport _countdownwidgetref 0)
        (if (not (Variables|/Game/Level1/Inventory/Items/BP_Countdown_Clock.BP_Countdown_Clock_C|GetIsCountingDown _countdown_clock))
          (Default|SetDuration _countdown_clock 1.2e+02)
          (Variables|/Game/Level1/Inventory/Items/BP_Countdown_Clock.BP_Countdown_Clock_C|SetIsCountingDown _countdown_clock true)
          (Variables|/Game/FirstPerson/Blueprints/BP_FirstPersonCharacter.BP_FirstPersonCharacter_C|SetHasStarted (Variables|Default|GetAs%20BP%20First%20Person%20Character) true))))))

(event EventBeginPlay
  (bind _asbp_dialogue_sys (Utilities|Casting|CastToBP_Dialogue_Sys (Game|GetPlayerController 0)))
  (Variables|Default|SetAs%20BP%20Dialogue%20Sys _asbp_dialogue_sys)
  (bind _asbp_first_person_character (Utilities|Casting|CastToBP_FirstPersonCharacter (Game|Player|GetPlayerPawn 0)))
  (Variables|Default|SetAs%20BP%20First%20Person%20Character _asbp_first_person_character)
  (bind _returnvalue (UserInterface|CreateWidget "/Game/Level1/Countdown/BP_CountdownTimer.BP_CountdownTimer_C"))
  (Variables|Default|SetCountdownWidgetRef _returnvalue)
  (bind _outactors (Actor|GetAllActorsOfClass "/Game/Level1/Inventory/Items/BP_Countdown_Clock.BP_Countdown_Clock_C"))
  (Variables|Default|SetCountdown%20Clock (Utilities|Array|Get(acopy) _outactors)))

(fn ConstructionScript)