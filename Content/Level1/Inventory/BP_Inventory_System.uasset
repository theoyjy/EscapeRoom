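; Inventory component for the first-person character that handles item storage and interaction with looked-at actors.
; Each tick, a camera sphere trace updates the looked-at actor and prints its message; the interact input passes it through a server event to its item data component.
; AddToInventory fills a fixed slot array one unit at a time, using data table stack limits before empty slots.
; RemoveFromInventory is an empty stub; key 1 prints slot contents for debugging.
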(event Custom|Server_Interact
  (params (target :type Actor%20Object%20Reference))
  (bind _asbp_first_person_character (Utilities|Casting|CastToBP_FirstPersonCharacter (Components|GetOwner)))
  (Class|InteractionInterface|Interactwith(Message) (Actor|GetComponentbyClass target "/Game/Level1/Inventory/BP_Item_Data_Component.BP_Item_Data_Component_C") _asbp_first_person_character))

(event Input|EnhancedActionEvents|EnhancedInputActionIA_Interact
  (params (ActionValue :type Boolean) (ElapsedSeconds :type Float%20%28double-precision%29) (TriggeredSeconds :type Float%20%28double-precision%29) (InputAction :type Input%20Action%20Object%20Reference :default "/Game/Level1/Inventory/Input/Actions/IA_Interact.IA_Interact"))
  (bind _lookatactor (Variables|Default|GetLookAtActor)
    (:then
      (CallFunction|ServerInteract _lookatactor))
    (:else)))

(event EventTick
  (params (DeltaSeconds :type Float%20%28single-precision%29))
  (CallFunction|InteractionTrace))

(event EventBeginPlay
  ;[1 1 1] Comment
  (Utilities|Array|Resize (Variables|Default|GetContent) (Variables|Default|GetSize))
  (bind _asbp_first_person_character (Utilities|Casting|CastToBP_FirstPersonCharacter (Components|GetOwner)))
  (bind _asplayer_controller (Utilities|Casting|CastToPlayerController (Pawn|GetController _asbp_first_person_character)))
  (Utilities|IsValid (PlayerController|LocalPlayerSubsystems|GetEnhancedInputLocalPlayerSubsystem _asplayer_controller)
    (:Is%20Valid
      (Input|AddMappingContext (PlayerController|LocalPlayerSubsystems|GetEnhancedInputLocalPlayerSubsystem _asplayer_controller) "/Game/Level1/Inventory/Input/IMC_Inventory.IMC_Inventory" 0 "(bIgnoreAllPressedKeysUntilRelease=True,bForceImmediately=False,bNotifyUserSettings=False)"))))

(event Input|KeyboardEvents|1
  (params (Key :type Key%20Structure))
  (:Pressed
    (CallFunction|DEBUGPrintContent)))

(fn AddtoInventory
  (params (ItemID :type Name) (Quantity :type Integer))
  (bind (_hasemptyslots _index) (CallFunction|AnyEmptySlotAvailable))
  (LocalVariables|SetLocal_Quantity_Remaining Quantity)
  (while (and (> (LocalVariables|GetLocal_Quantity_Remaining) 0) (not (LocalVariables|GetLocal_HasFailed)))
    (bind (_index_2 _foundslot) (CallFunction|FindSlot ItemID))
    (if _foundslot
      (CallFunction|AddtoStack _index_2 1)
      (Math|Integer|DecrementInt (LocalVariables|GetLocal_Quantity_Remaining))
      (elif _hasemptyslots
        (CallFunction|CreateNewStack _index ItemID 1)
        (Math|Integer|DecrementInt (LocalVariables|GetLocal_Quantity_Remaining))
        (else
          (LocalVariables|SetLocal_HasFailed true)))))
  (Class|BackpackActorController|ControlUpdateBackpackItem)
  (return (not (LocalVariables|GetLocal_HasFailed)) (LocalVariables|GetLocal_Quantity_Remaining)))

(fn RemovefromInventory)

(fn InteractionTrace
  (bind _returnvalue (Game|GetPlayerCameraManager 0))
  (bind _returnvalue_2 (Transformation|GetActorLocation _returnvalue))
  (bind _outhit (Collision|SphereTraceByChannel _returnvalue_2 (+ _returnvalue_2 (* (Transformation|GetActorForwardVector _returnvalue) (Variables|Default|GetInteractionRange))) 15.0 "TraceTypeQuery3" false (Utilities|Array|MakeArray (Components|GetOwner)) "None"))
  (if true
    (if (!= (.HitActor (Collision|BreakHitResult _outhit)) (Variables|Default|GetLookAtActor))
      (bind _output_get (Variables|Default|SetLookAtActor (.HitActor (Collision|BreakHitResult _outhit))))
      (bind _message (Class|InteractionInterface|Lookat(Message) _output_get))
      (Development|PrintText _message))
    (else
      (Variables|Default|SetLookAtActor 0))))

(fn FindSlot
  (params (ItemID :type Name))
  (for (_array_element _array_index) (Variables|Default|GetContent)
    (if (== (.ItemID (Utilities|Struct|BreakBP_Slot_Struct _array_element)) ItemID)
      (if (< (.Quantity (Utilities|Struct|BreakBP_Slot_Struct _array_element)) (CallFunction|GetMaxStackSize ItemID))
        (return _array_index true))))
  (return -1 false))

(fn GetMaxStackSize
  (params (ItemID :type Name))
  (bind _returnvalue (Utilities|GetDataTableRow "/Game/Level1/Inventory/BP_Item_Data.BP_Item_Data" ItemID)
    (:then
      (return (.StackSize (Utilities|Struct|BreakBP_Item_Struct _returnvalue))))
    (:RowNotFound
      (return -1))))

(fn AddtoStack
  (params (Index :type Integer) (Quantity :type Integer))
  (bind _content (Variables|Default|GetContent))
  (bind _output (Utilities|Array|Get(acopy) _content Index))
  (bind (_itemid _quantity) (Utilities|Struct|BreakBP_Slot_Struct _output))
  (Utilities|Array|SetArrayElem (Variables|Default|GetContent) Index (Utilities|Struct|MakeBP_Slot_Struct _itemid (+ _quantity Quantity))))

(fn AnyEmptySlotAvailable
  (for (_array_element _array_index) (Variables|Default|GetContent)
    (if (== (.Quantity (Utilities|Struct|BreakBP_Slot_Struct _array_element)) 0)
      (return true _array_index)))
  (return false -1))

(fn CreateNewStack
  (params (Index :type Integer) (ItemID :type Name) (Quantity :type Integer))
  (Utilities|Array|SetArrayElem (Variables|Default|GetContent) Index (Utilities|Struct|MakeBP_Slot_Struct ItemID Quantity)))

(fn DEBUGPrintContent
  (for (_array_element _array_index) (Variables|Default|GetContent)
    (Development|PrintString (Utilities|String|Append (Utilities|String|ToString(Integer) _array_index) " : " (Utilities|String|ToString(Name) (.ItemID (Utilities|Struct|BreakBP_Slot_Struct _array_element))) " = " (Utilities|String|ToString(Integer) (.Quantity (Utilities|Struct|BreakBP_Slot_Struct _array_element)))))))