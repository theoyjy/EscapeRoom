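; BP_Item_Data_Component is an item component that lets its owning actor be picked up into the player's inventory.
; Interactwith checks the first-person character's IsItem flag, then passes the item's row name and quantity to the interacting player's BPInventorySystem.
; GetIsItem matches a name against that row name, and LookAt returns an empty string.
; A successful add leaves the actor in place, as the DestroyActor call is unconnected.
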(event EventInteractwith
  (params (PlayerCharacter :type BP%20First%20Person%20Character%20Object%20Reference))
  (bind _bp_inventory_system (Variables|/Game/FirstPerson/Blueprints/BP_FirstPersonCharacter.BP_FirstPersonCharacter_C|GetBP_Inventory_System PlayerCharacter))
  (bind _asbp_first_person_character (Utilities|Casting|CastToBP_FirstPersonCharacter (Game|GetPlayerCharacter 0)))
  (if (Variables|/Game/FirstPerson/Blueprints/BP_FirstPersonCharacter.BP_FirstPersonCharacter_C|GetIsItem _asbp_first_person_character)
    (Utilities|IsValid _bp_inventory_system
      (:Is%20Valid
        (bind _success (Default|AddtoInventory _bp_inventory_system (.RowName (Utilities|Struct|BreakDataTableRowHandle (Variables|Default|GetItemID))) (Variables|Default|GetQuantity)))
        (if _success
          _)))))

(fn GetIsItem
  (params (Name :type String))
  (return (== Name (.RowName (Utilities|Struct|BreakDataTableRowHandle (Variables|Default|GetItemID))))))

(fn Lookat
  (return ""))