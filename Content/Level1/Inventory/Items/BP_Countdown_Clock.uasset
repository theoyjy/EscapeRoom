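; BP_Countdown_Clock is a countdown clock that shows its remaining time on a TextRender component.
; SetDuration stores the countdown length, and Tick calls StartCountdown, which subtracts frame delta time while IsCountingDown is true.
; The display trims the last character of the formatted time to show tenths of a second.
; At zero it stops, restores the stored duration and displays a zeroed time.
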(event Custom|SetDuration
  (params (NewCountdownDuration :type Float%20%28double-precision%29))
  (bind _output_get (Variables|Default|SetCurrentTime NewCountdownDuration))
  (Variables|Default|SetCountdownDuration _output_get))

(event Custom|StartCountdown
  (if (Variables|Default|GetIsCountingDown)
    (bind _output_get (Variables|Default|SetCurrentTime (Math|Float|Clamp(Float) (- (Variables|Default|GetCurrentTime) (Utilities|Time|GetWorldDeltaSeconds)) 0.0 (Variables|Default|GetCurrentTime))))
    (Rendering|Components|TextRender|SetText (Variables|Default|GetTextRender) (Utilities|Text|ToText(String) (Utilities|String|LeftChop (Class|KismetStringLibrary|TimeSecondstoString _output_get) 1)))
    (if (<= (Variables|Default|GetCurrentTime) 0.0)
      (Variables|Default|SetIsCountingDown false)
      (Variables|Default|SetCurrentTime (Variables|Default|GetCountdownDuration))
      (Variables|Default|SetNewVar "00:00.0")
      (Rendering|Components|TextRender|SetText (Variables|Default|GetTextRender) (Utilities|Text|ToText(String) (Variables|Default|GetNewVar))))))

(event EventTick
  (params (DeltaSeconds :type Float%20%28single-precision%29))
  (CallFunction|StartCountdown))

(fn ConstructionScript)