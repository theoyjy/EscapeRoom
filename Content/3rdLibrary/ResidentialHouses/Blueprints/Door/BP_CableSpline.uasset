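; Cable spline Blueprint that builds a sagging or tensioned cable between a start and end point in the construction script.
; A middle spline point is interpolated in X and Y by TensionPointPosition, with Tension setting its local Z height.
; Spline mesh components are generated at MeshLength intervals with the chosen mesh and material, using length-scaled tangents sampled along the spline.
; Endpoint tangents are recomputed from neighbouring point tangents inside the segment loop.
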(fn ConstructionScript
  (bind _returnvalue (Math|Vector|VectorZero))
  (bind _cablespline (Variables|Default|GetCableSpline))
  (bind _cablespline_2 (Variables|Default|GetCableSpline))
  (bind _returnvalue_2 (Spline|GetTangentatSplinePoint _cablespline_2 1 "Local"))
  (bind _p (Utilities|GetCenter))
  (bind _output_get (Variables|Default|SetSplinePointArray (Utilities|Array|MakeArray (Variables|Default|GetStart%20Point) _p (Variables|Default|GetEndPoint))))
  (Spline|SetSplinePoints (Variables|Default|GetCableSpline) _output_get "Local" true)
  (for _index (range -2 (- (.ReturnValue (Math|Float|Division(WholeandRemainder) (Spline|GetSplineLength (Variables|Default|GetCableSpline)) (Variables|Default|GetMeshLength))) 0))
    (bind (_startpos _starttangent _endpos _endtangent) (CallFunction|SplineIndexPos (Variables|Default|GetCableSpline) _index))
    ;[1 0.07113 0] Setting start and end points tangents to point towards center
    (Spline|SetTangentsatSplinePoint _cablespline 2 (Math|Vector|Normalize (- (Spline|GetTangentatSplinePoint _cablespline_2 2 "Local") _returnvalue_2)) _returnvalue "Local" true)
    (Spline|SetTangentsatSplinePoint _cablespline 0 _returnvalue (Math|Vector|Normalize (- _returnvalue_2 (Spline|GetTangentatSplinePoint _cablespline_2 0 "Local"))) "Local" true)
    (bind _returnvalue_3 (AddComponent|AddSplineMeshComponent false))
    (Components|StaticMesh|SetStaticMesh _returnvalue_3 (Variables|Default|GetMesh))
    (Rendering|Material|SetMaterial _returnvalue_3 0 (Variables|Default|GetMaterial))
    (SplineMesh|SetStartandEnd _returnvalue_3 _startpos _starttangent _endpos _endtangent true :!class /Script/Engine.SplineMeshComponent)))

(fn SplineIndexPos
  (params (Spline :type Spline%20Component%20Object%20Reference) (Index :type Integer))
  (bind _returnvalue (+ Index 1))
  (bind _meshlength (Variables|Default|GetMeshLength))
  (bind _meshlength_2 (Variables|Default|GetMeshLength))
  (bind _returnvalue_2 (* Index _meshlength_2))
  (bind _returnvalue_3 (* _returnvalue _meshlength))
  (return (Spline|GetLocationatDistanceAlongSpline Spline _returnvalue_2 "Local") (* (Math|Vector|Normalize (Spline|GetTangentatDistanceAlongSpline Spline _returnvalue_2 "Local")) (Variables|Default|GetMeshLength)) (Spline|GetLocationatDistanceAlongSpline Spline _returnvalue_3 "Local") (* (Math|Vector|Normalize (Spline|GetTangentatDistanceAlongSpline Spline _returnvalue_3 "Local")) (Variables|Default|GetMeshLength))))