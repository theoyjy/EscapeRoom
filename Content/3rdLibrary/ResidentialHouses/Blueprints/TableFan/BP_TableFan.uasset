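; Table fan prop with spinning blades, an oscillating head and audio, configured by a speed setting.
; BeginPlay maps the FanSpeed enum to off or one of three blade and swing rates.
; RotationTimeline swings Top and drives FanTimeLine from its update to spin the blades, using near-yaw checks at either limit to reverse or restart the sweep.
; The construction script sets arm tilt, plus head yaw when TurnOff is set.
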(event EventBeginPlay
  ;[0.06258 0.03314 0.1719] FanStates
  (if (Utilities|Enum|Equal(Enum) (Variables|Default|GetFanSpeed) "NewEnumerator0")
    (Variables|Default|SetTurn%20Off true)
    (Variables|Default|SetSwingSpeed 0.0)
    (elif (Utilities|Enum|Equal(Enum) (Variables|Default|GetFanSpeed) "NewEnumerator1")
      (Variables|Default|SetFanSpeedCount 3.0)
      (Variables|Default|SetTurn%20Off false)
      (Variables|Default|SetSwingSpeed 0.5)
      ;[0.06258 0.03314 0.1719] Play Audio
      (Audio|Components|Audio|Play (Variables|Default|GetAudio) 0.0 :!label _label)
      ;[0.06258 0.03314 0.1719] Check On/Off
      (if (Variables|Default|GetTurn%20Off)
        ;[0.06258 0.03314 0.1719] Rotate |TOP| with Timeline
        (bind _rotation (Timeline|RotationTimeline Stop)
          (:Update
            (Transformation|SetRelativeRotation (Variables|Default|GetTop) (Math|Rotator|MakeRotator 0.0 0.0 _rotation) false false)
            ;[0.06258 0.03314 0.1719] Fan Rotate Timeline
            (Components|Timeline|SetPlayRate (Variables|Default|GetFanTimeLine) (Variables|Default|GetFanSpeedCount))
            (bind _rotation_2 (Timeline|FanTimeLine Play)
              (:Update
                (Transformation|SetRelativeRotation (Variables|Default|GetFan) (Math|Rotator|MakeRotator _rotation_2 0.0 0.0) false false)
                ;[0.06258 0.03314 0.1719] Check if Rotation is Nearly B
                (if (Math|Float|NearlyEqual(Float) (.yaw (Variables|/Script/Engine.SceneComponent|GetRelativeRotation (Variables|Default|GetTop))) -5e+01 1.0)
                  (Timeline|RotationTimeline Reverse)))))
          (:Finished
            (if (Math|Float|NearlyEqual(Float) (.yaw (Variables|/Script/Engine.SceneComponent|GetRelativeRotation (Variables|Default|GetTop))) 5e+01 1.0)
              (Timeline|RotationTimeline PlayFromStart))))
        (else
          ;[0.06258 0.03314 0.1719] Timeline PlayRate
          (Components|Timeline|SetPlayRate (Variables|Default|GetRotationTimeline) (Variables|Default|GetSwingSpeed))
          (Timeline|RotationTimeline Play)))
      (elif (Utilities|Enum|Equal(Enum) (Variables|Default|GetFanSpeed) "NewEnumerator2")
        (Variables|Default|SetFanSpeedCount 6.0)
        (Variables|Default|SetTurn%20Off false)
        (Variables|Default|SetSwingSpeed 1.0)
        (goto _label)
        (elif (Utilities|Enum|Equal(Enum) (Variables|Default|GetFanSpeed) "NewEnumerator3")
          (Variables|Default|SetFanSpeedCount 9.0)
          (Variables|Default|SetTurn%20Off false)
          (Variables|Default|SetSwingSpeed 1.5)
          (goto _label))))))

(fn ConstructionScript
  (Transformation|SetRelativeRotation (Variables|Default|GetArm) (Math|Rotator|MakeRotator 0.0 (Variables|Default|GetAngle) 0.0) false false)
  (if (Variables|Default|GetTurn%20Off)
    (Transformation|SetRelativeRotation (Variables|Default|GetTop) (Math|Rotator|MakeRotator 0.0 0.0 (Variables|Default|GetRotation)) false false)))