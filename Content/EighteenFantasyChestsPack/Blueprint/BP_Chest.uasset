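; BP_Chest is an openable chest with eighteen selectable styles that the player opens with F.
; The construction script uses ChestIndex to pick body and lid meshes and lid height, and applies a preset LidAngle.
; While LidAngle is zero, box overlap toggles actor input and a prompt widget.
; F removes the prompt and plays a timeline that rolls the lid open, updating LidAngle.
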(event OnComponentBeginOverlap(Box)
  (params (OverlappedComponent :type Primitive%20Component%20Object%20Reference) (OtherActor :type Actor%20Object%20Reference) (OtherComp :type Primitive%20Component%20Object%20Reference) (OtherBodyIndex :type Integer) (bFromSweep :type Boolean) (SweepResult :type Hit%20Result%20Structure%20%28by%20ref%29))
  ;[0 0 0] Enable input when the player overlaps the collision box
  (if (and (or (== OtherActor (Game|GetPlayerCharacter 0)) (== OtherActor (Game|Player|GetPlayerPawn 0))) (== (Variables|Default|GetLidAngle) 0.0))
    (Input|EnableInput (Game|GetPlayerController 0))
    (bind _returnvalue (UserInterface|CreateWidget "/Game/EighteenFantasyChestsPack/UI/Widget_ChestInteraction.Widget_ChestInteraction_C"))
    (UserInterface|Viewport|AddtoViewport _returnvalue 0)
    (Variables|Default|SetChestInteractionWidget _returnvalue)))

(event OnComponentEndOverlap(Box)
  (params (OverlappedComponent :type Primitive%20Component%20Object%20Reference) (OtherActor :type Actor%20Object%20Reference) (OtherComp :type Primitive%20Component%20Object%20Reference) (OtherBodyIndex :type Integer))
  (bind _chestinteractionwidget (Variables|Default|GetChestInteractionWidget))
  ;[0 0 0] Disable input when the player stops overlapping the collision box
  (if (and (or (== OtherActor (Game|GetPlayerCharacter 0)) (== OtherActor (Game|Player|GetPlayerPawn 0))) (== (Variables|Default|GetLidAngle) 0.0))
    (Input|DisableInput (Game|GetPlayerController 0))
    (Utilities|IsValid _chestinteractionwidget
      (:Is%20Valid
        (Widget|RemovefromParent _chestinteractionwidget)))))

(event Input|KeyboardEvents|F
  (params (Key :type Key%20Structure :default "None"))
  (bind _chestlid (Variables|Default|GetChestLid))
  (bind _relativerotation (Variables|/Script/Engine.SceneComponent|GetRelativeRotation _chestlid))
  ;[0 0 0] Open chest when the player press the F button
  (:Pressed
    (if (== (Variables|Default|GetLidAngle) 0.0)
      (Widget|RemovefromParent (Variables|Default|GetChestInteractionWidget))
      (bind _lidrotation (Timeline|OpeningChestTimeline Play)
        (:Update
          (bind _output_get (Variables|Default|SetLidAngle _lidrotation))
          (Transformation|SetRelativeRotation _chestlid (Math|Rotator|MakeRotator _output_get (.pitch _relativerotation) (.yaw _relativerotation)) false false))))))

(fn ConstructionScript
  (bind _chestlid (Variables|Default|GetChestLid))
  (bind _chestindex (Variables|Default|GetChestIndex))
  (bind _chestlid_2 (Variables|Default|GetChestLid))
  (bind _relativelocation (Variables|/Script/Engine.SceneComponent|GetRelativeLocation _chestlid_2))
  (bind _relativerotation (Variables|/Script/Engine.SceneComponent|GetRelativeRotation _chestlid))
  (Utilities|FlowControl|Sequence
    (:then_0
      ;[0 0 0] Custom rotation of the lid
      (Transformation|SetRelativeRotation (Variables|Default|GetChestLid) (Math|Rotator|MakeRotator (Variables|Default|GetLidAngle) (.pitch _relativerotation) (.yaw _relativerotation)) false false))
    (:then_1
      ;[0 0 0] Change chest type
      (Transformation|SetRelativeLocation _chestlid_2 (Math|Vector|MakeVector (.x _relativelocation) (.y _relativelocation) (Utilities|Select :Index _chestindex :Option%200 5e+01 :Option%201 6e+01 :Option%202 4e+01 :Option%203 6e+01 :Option%204 5e+01 :Option%205 6e+01 :Option%206 5e+01 :Option%207 6e+01 :Option%208 7e+01 :Option%209 6e+01 :Option%2010 6e+01 :Option%2011 6e+01 :Option%2012 6e+01 :Option%2013 4e+01 :Option%2014 6e+01 :Option%2015 6e+01 :Option%2016 5e+01 :Option%2017 6e+01)) false false)
      (Components|StaticMesh|SetStaticMesh (Variables|Default|GetChest) (Utilities|Select :Index _chestindex :Option%200 "/Game/EighteenFantasyChestsPack/StaticMeshes/SM_ClassicalChest.SM_ClassicalChest" :Option%201 "/Game/EighteenFantasyChestsPack/StaticMeshes/SM_FortifiedChest.SM_FortifiedChest" :Option%202 "/Game/EighteenFantasyChestsPack/StaticMeshes/SM_ChestOfAphrodite.SM_ChestOfAphrodite" :Option%203 "/Game/EighteenFantasyChestsPack/StaticMeshes/SM_ChestWithGoldenEdging.SM_ChestWithGoldenEdging" :Option%204 "/Game/EighteenFantasyChestsPack/StaticMeshes/SM_ChurchChest.SM_ChurchChest" :Option%205 "/Game/EighteenFantasyChestsPack/StaticMeshes/SM_CurvedChest.SM_CurvedChest" :Option%206 "/Game/EighteenFantasyChestsPack/StaticMeshes/SM_DemonicChest.SM_DemonicChest" :Option%207 "/Game/EighteenFantasyChestsPack/StaticMeshes/SM_DragonChest.SM_DragonChest" :Option%208 "/Game/EighteenFantasyChestsPack/StaticMeshes/SM_DruidChest.SM_DruidChest" :Option%209 "/Game/EighteenFantasyChestsPack/StaticMeshes/SM_ElvenChest_.SM_ElvenChest_" :Option%2010 "/Game/EighteenFantasyChestsPack/StaticMeshes/SM_GothicChest.SM_GothicChest" :Option%2011 "/Game/EighteenFantasyChestsPack/StaticMeshes/SM_GreekChest.SM_GreekChest" :Option%2012 "/Game/EighteenFantasyChestsPack/StaticMeshes/SM_JapaneseChest.SM_JapaneseChest" :Option%2013 "/Game/EighteenFantasyChestsPack/StaticMeshes/SM_NecromancerChest.SM_NecromancerChest" :Option%2014 "/Game/EighteenFantasyChestsPack/StaticMeshes/SM_PirateChest.SM_PirateChest" :Option%2015 "/Game/EighteenFantasyChestsPack/StaticMeshes/SM_StoneChest.SM_StoneChest" :Option%2016 "/Game/EighteenFantasyChestsPack/StaticMeshes/SM_VampireChest.SM_VampireChest" :Option%2017 "/Game/EighteenFantasyChestsPack/StaticMeshes/SM_VikingChest.SM_VikingChest"))
      (Components|StaticMesh|SetStaticMesh (Variables|Default|GetChestLid) (Utilities|Select :Index _chestindex :Option%200 "/Game/EighteenFantasyChestsPack/StaticMeshes/SM_ClassicalChest_Lid.SM_ClassicalChest_Lid" :Option%201 "/Game/EighteenFantasyChestsPack/StaticMeshes/SM_FortifiedChest_Lid.SM_FortifiedChest_Lid" :Option%202 "/Game/EighteenFantasyChestsPack/StaticMeshes/SM_ChestOfAphrodite_Lid.SM_ChestOfAphrodite_Lid" :Option%203 "/Game/EighteenFantasyChestsPack/StaticMeshes/SM_ChestWithGoldenEdging_Lid.SM_ChestWithGoldenEdging_Lid" :Option%204 "/Game/EighteenFantasyChestsPack/StaticMeshes/SM_ChurchChest_Lid.SM_ChurchChest_Lid" :Option%205 "/Game/EighteenFantasyChestsPack/StaticMeshes/SM_CurvedChest_Lid.SM_CurvedChest_Lid" :Option%206 "/Game/EighteenFantasyChestsPack/StaticMeshes/SM_DemonicChest_Lid.SM_DemonicChest_Lid" :Option%207 "/Game/EighteenFantasyChestsPack/StaticMeshes/SM_DragonChest_Lid.SM_DragonChest_Lid" :Option%208 "/Game/EighteenFantasyChestsPack/StaticMeshes/SM_DruidChest_Lid.SM_DruidChest_Lid" :Option%209 "/Game/EighteenFantasyChestsPack/StaticMeshes/SM_ElvenChest_Lid.SM_ElvenChest_Lid" :Option%2010 "/Game/EighteenFantasyChestsPack/StaticMeshes/SM_GothicChest_Lid.SM_GothicChest_Lid" :Option%2011 "/Game/EighteenFantasyChestsPack/StaticMeshes/SM_GreekChest_Lid.SM_GreekChest_Lid" :Option%2012 "/Game/EighteenFantasyChestsPack/StaticMeshes/SM_JapaneseChest_Lid.SM_JapaneseChest_Lid" :Option%2013 "/Game/EighteenFantasyChestsPack/StaticMeshes/SM_NecromancerChest_Lid.SM_NecromancerChest_Lid" :Option%2014 "/Game/EighteenFantasyChestsPack/StaticMeshes/SM_PirateChest_Lid.SM_PirateChest_Lid" :Option%2015 "/Game/EighteenFantasyChestsPack/StaticMeshes/SM_StoneChest_Lid.SM_StoneChest_Lid" :Option%2016 "/Game/EighteenFantasyChestsPack/StaticMeshes/SM_VampireChest_Lid.SM_VampireChest_Lid" :Option%2017 "/Game/EighteenFantasyChestsPack/StaticMeshes/SM_VikingChest_Lid.SM_VikingChest_Lid")))))