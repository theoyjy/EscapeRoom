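; Password-locked chest that shows an interaction prompt and accepts input while the player overlaps its box and the lid is closed.
; Pressing F opens the password widget in UI-only mode with a cursor.
; Tick polls CodeCorrected, which is set outside this graph, then flags IsChestOpen on the first-person character, rotates the lid via timeline and restores game input.
; The construction script sets classical chest meshes and initial lid transform.
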(event OnComponentBeginOverlap(Box)
  (params (OverlappedComponent :type Primitive%20Component%20Object%20Reference) (OtherActor :type Actor%20Object%20Reference) (OtherComp :type Primitive%20Component%20Object%20Reference) (OtherBodyIndex :type Integer) (bFromSweep :type Boolean) (SweepResult :type Hit%20Result%20Structure%20%28by%20ref%29))
  ;[0 0 0] Enable input when the player overlaps the collision box
  (if (and (or (== OtherActor (Game|GetPlayerCharacter 0)) (== OtherActor (Game|Player|GetPlayerPawn 0))) (== (Variables|Default|GetLidAngle) 0.0))
    (Input|EnableInput (Game|GetPlayerController 0))
    (bind _returnvalue (UserInterface|CreateWidget "/Game/EighteenFantasyChestsPack/UI/Widget_ChestInteraction.Widget_ChestInteraction_C"))
    (UserInterface|Viewport|AddtoViewport _returnvalue 0)
    (Variables|Default|SetChestInteractionWidget _returnvalue)))

(event OnComponentEndOverlap(Box)
  (params (OverlappedComponent :type Primitive%20Component%20Object%20Reference) (OtherActor :type Actor%20Object%20Reference) (OtherComp :type Primitive%20Component%20Object%20Reference) (OtherBodyIndex :type Integer))
  (bind _chestinteractionwidget (Variables|Default|GetChestInteractionWidget))
  ;[0 0 0] Disable input when the player stops overlapping the collision box
  (if (and (or (== OtherActor (Game|GetPlayerCharacter 0)) (== OtherActor (Game|Player|GetPlayerPawn 0))) (== (Variables|Default|GetLidAngle) 0.0))
    (Input|DisableInput (Game|GetPlayerController 0))
    (Utilities|IsValid _chestinteractionwidget
      (:Is%20Valid
        (Widget|RemovefromParent _chestinteractionwidget)))))

(event EventTick
  (params (DeltaSeconds :type Float%20%28single-precision%29))
  (bind _returnvalue (Game|GetPlayerController 0))
  (bind _chestlid (Variables|Default|GetChestLid))
  (bind _relativerotation (Variables|/Script/Engine.SceneComponent|GetRelativeRotation _chestlid))
  ;[0 0 0] Open chest when the player press the F button
  (if (Variables|Default|GetCodeCorrected?)
    (Variables|Default|SetCodeCorrected? false)
    (bind _asbp_first_person_character (Utilities|Casting|CastToBP_FirstPersonCharacter (Game|GetPlayerCharacter 0)))
    (Development|PrintString "Chest Opened")
    (Variables|/Game/FirstPerson/Blueprints/BP_FirstPersonCharacter.BP_FirstPersonCharacter_C|SetIsChestOpen _asbp_first_person_character true)
    (Widget|RemovefromParent (Variables|Default|GetChestInteractionWidget))
    (bind _lidrotation (Timeline|OpeningChestTimeline Play)
      (:Update
        (bind _output_get (Variables|Default|SetLidAngle _lidrotation))
        (Transformation|SetRelativeRotation _chestlid (Math|Rotator|MakeRotator _output_get (.pitch _relativerotation) (.yaw _relativerotation)) false false)
        (Variables|/Script/Engine.PlayerController|SetbShowMouseCursor _returnvalue false)
        (Input|SetInputModeGameOnly _returnvalue false)))))

(event Input|KeyboardEvents|F
  (params (Key :type Key%20Structure))
  (bind _returnvalue (Game|GetPlayerController 0))
  ;[0 0 0] Open chest when the player press the F button
  (:Pressed
    (if (== (Variables|Default|GetLidAngle) 0.0)
      (Input|EnableInput _returnvalue)
      (bind _returnvalue_2 (UserInterface|CreateWidget "/Game/FirstPerson/Blueprints/UI_Password_New.UI_Password_New_C"))
      (UserInterface|Viewport|AddtoViewport _returnvalue_2 100)
      (Variables|/Script/Engine.PlayerController|SetbShowMouseCursor _returnvalue true)
      (Input|SetInputModeUIOnly _returnvalue _returnvalue_2 "DoNotLock" true))))

(fn ConstructionScript
  (bind _chestlid (Variables|Default|GetChestLid))
  (bind _chestlid_2 (Variables|Default|GetChestLid))
  (bind _relativelocation (Variables|/Script/Engine.SceneComponent|GetRelativeLocation _chestlid_2))
  (bind _relativerotation (Variables|/Script/Engine.SceneComponent|GetRelativeRotation _chestlid))
  (Utilities|FlowControl|Sequence
    (:then_0
      ;[0 0 0] Custom rotation of the lid
      (Transformation|SetRelativeRotation (Variables|Default|GetChestLid) (Math|Rotator|MakeRotator (Variables|Default|GetLidAngle) (.pitch _relativerotation) (.yaw _relativerotation)) false false))
    (:then_1
      ;[0 0 0] Change chest type
      (Transformation|SetRelativeLocation _chestlid_2 (Math|Vector|MakeVector (.x _relativelocation) (.y _relativelocation) 5e+01) false false)
      (Components|StaticMesh|SetStaticMesh (Variables|Default|GetChest) "/Game/EighteenFantasyChestsPack/StaticMeshes/SM_ClassicalChest.SM_ClassicalChest")
      (Components|StaticMesh|SetStaticMesh (Variables|Default|GetChestLid) "/Game/EighteenFantasyChestsPack/StaticMeshes/SM_ClassicalChest_Lid.SM_ClassicalChest_Lid"))))